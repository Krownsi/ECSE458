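; BP_SpaceShip is a drivable spaceship with two switchable views.
; The Drive axis applies an impulse to the Pod along RootArrow's forward vector, scaled by the axis value and DrivePower, so movement is physics-driven.
; The ToggleCameraView action uses a FlipFlop to alternate which of ViewA and ViewB is active.
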(event Input|ActionEvents|InputActionToggleCameraView
  (params (Key :type Key%20Structure :default "None"))
  (bind _viewa (Variables|Components|GetViewA))
  (bind _viewb (Variables|Default|GetViewB))
  ;[1 1 1] Handles Toggling of Camera Views
  (:Pressed
    (Utilities|FlowControl|FlipFlop
      (:A
        (Components|Activation|Activate _viewa false)
        (Components|Activation|Deactivate _viewb))
      (:B
        (Components|Activation|Activate _viewb false)
        (Components|Activation|Deactivate _viewa)))))

(event Input|AxisEvents|InputAxisDrive
  (params (AxisValue :type Float%20%28single-precision%29))
  (Physics|AddImpulse (Variables|Components|GetPod) (* (Math|Vector|GetForwardVector (Transformation|GetWorldRotation (Variables|Default|GetRootArrow))) (* AxisValue (Variables|Default|GetDrivePower))) "None" false))

(fn ConstructionScript)